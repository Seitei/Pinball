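; BP_Rail is a spline-driven rail actor that builds its geometry from mesh segments along an editable path.
; The Construction Script adds one spline mesh component per span between spline points, using start, middle or end meshes according to position.
; Each segment bends to the local locations and tangents of its two bounding points.
; BeginPlay is empty, and a start-scale step is left unconnected.
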(event `self.ReceiveBeginPlay`)

(fn `UserConstructionScript`
  (bind _spline (`self.Spline`))
  (bind _returnvalue (- (`SplineComponent.GetNumberOfSplinePoints` (`self.Spline`)) 2))
  (for _index (range (+ _returnvalue 1))
    (bind _returnvalue_2 (`AddComponent|NODE_AddSplineMeshComponent-0`))
    (if (== _index 0)
      (`StaticMeshComponent.SetStaticMesh` _returnvalue_2 (`self.RailStartMesh`))
      (elif (== _returnvalue _index)
        (`StaticMeshComponent.SetStaticMesh` _returnvalue_2 (`self.RailEndMesh`))
        (else
          (`StaticMeshComponent.SetStaticMesh` _returnvalue_2 (`self.RailMidMesh`)))))
    (bind (_location _tangent) (`SplineComponent.GetLocationAndTangentAtSplinePoint` _spline _index "Local"))
    (bind (_location_2 _tangent_2) (`SplineComponent.GetLocationAndTangentAtSplinePoint` _spline (+ _index 1) "Local"))
    (`SplineMeshComponent.SetStartAndEnd` _returnvalue_2 _location _tangent _location_2 _tangent_2 true)))