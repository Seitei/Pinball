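; ForceMovementZone is a zone actor that steers overlapping BP_ball actors along the direction of its Arrow component.
; Every tick it converts each ball's velocity into the arrow's local space and interpolates it toward a forward-only velocity with a clamped speed, at AdoptionSpeed.
; The result returns to world space and replaces the ball's physics linear velocity, gradually removing sideways drift and enforcing forward motion.
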(event `self.ReceiveTick`
  (params (DeltaSeconds :type "Float (single-precision)"))
  (for _array_element (`self.GetOverlappingActors` "/Game/Blueprints/BP_ball.BP_ball_C")
    (bind _returnvalue (`KismetMathLibrary.InverseTransformDirection` (`SceneComponent.K2_GetComponentToWorld` (`self.Arrow`)) (`self.GetVelocity` _array_element)))
    (`PrimitiveComponent.SetPhysicsLinearVelocity` (`/Game/Blueprints/BP_ball.Ball` (cast `/Game/Blueprints/BP_ball` _array_element :!pure true)) (`KismetMathLibrary.TransformDirection` (`SceneComponent.K2_GetComponentToWorld` (`self.Arrow`)) (`KismetMathLibrary.VInterpTo` _returnvalue (`KismetMathLibrary.MakeVector` (`KismetMathLibrary.FClamp` (.x _returnvalue) 800.0 19000.0)) (`GameplayStatics.GetWorldDeltaSeconds`) (`self.AdoptionSpeed`))) false "None")))

(fn `UserConstructionScript`)